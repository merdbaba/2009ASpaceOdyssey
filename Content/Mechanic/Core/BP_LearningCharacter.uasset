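; Player character for a learning project that shows minimap and mission HUD widgets and lets the player interact with objects in view.
; Interact and Computer inputs each line trace from the follow camera, then call Interact on a hit BP_InteractActor or, after a brief delay, BP_ComputerActive.
; Failed traces or casts print debug messages.
; UpdateMission stores the current mission and writes it to the mission widget's text.
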(event Input|EnhancedActionEvents|EnhancedInputActionIA_Interact
  (params (ActionValue :type Boolean) (ElapsedSeconds :type Float%20%28double-precision%29) (TriggeredSeconds :type Float%20%28double-precision%29) (InputAction :type Input%20Action%20Object%20Reference :default "/Game/Mechanic/Input/IA_Interact.IA_Interact"))
  (bind _followcamera (Variables|Default|GetFollowCamera))
  (bind _returnvalue (Transformation|GetWorldLocation _followcamera))
  (:Started
    (bind (_outhit _returnvalue_2) (Collision|LineTraceByChannel _returnvalue (+ _returnvalue (* (Math|Vector|GetForwardVector _followcamera) 600)) "TraceTypeQuery1" false 0 "None"))
    (if _returnvalue_2
      (bind _asbp_interact_actor (Utilities|Casting|CastToBP_InteractActor (.HitActor (Collision|BreakHitResult _outhit)))
        (:then
          (Default|Interact _asbp_interact_actor))
        (:CastFailed
          (Development|PrintString "There is no interaction")))
      (else
        (Development|PrintString "no hit" true true "(R=0.000000,G=1.000000,B=0.065826,A=1.000000)")))))

(event Input|EnhancedActionEvents|EnhancedInputActionIA_Computer
  (params (ActionValue :type Boolean) (ElapsedSeconds :type Float%20%28double-precision%29) (TriggeredSeconds :type Float%20%28double-precision%29) (InputAction :type Input%20Action%20Object%20Reference :default "/Game/Mechanic/Input/IA_Computer.IA_Computer"))
  (bind _followcamera (Variables|Default|GetFollowCamera))
  (bind _returnvalue (Transformation|GetWorldLocation _followcamera))
  (bind (_outhit _returnvalue_2) (Collision|LineTraceByChannel _returnvalue (+ _returnvalue (* (Math|Vector|GetForwardVector _followcamera) 600)) "TraceTypeQuery1" false 0 "None"))
  (if _returnvalue_2
    (Utilities|FlowControl|Delay 0.12)
    (bind _asbp_computer_active (Utilities|Casting|CastToBP_ComputerActive (.HitActor (Collision|BreakHitResult _outhit)))
      (:then
        (Default|Interact _asbp_computer_active))
      (:CastFailed
        (Development|PrintString "There is no interaction")))
    (else
      (Development|PrintString "no hit" true true "(R=0.000000,G=1.000000,B=0.065826,A=1.000000)"))))

(event EventBeginPlay
  (|CallParentFunction)
  (bind _returnvalue (UserInterface|CreateWidget "/Game/Mechanic/Minimap/WBP_MiniMap.WBP_MiniMap_C" (Game|GetPlayerController 0)))
  (UserInterface|Viewport|AddtoViewport _returnvalue 0)
  (bind _returnvalue_2 (UserInterface|CreateWidget "/Game/Mechanic/Missions/WBP_Mission.WBP_Mission_C" (Game|GetPlayerController 0)))
  (bind _output_get (Variables|Default|SetMissionWBP _returnvalue_2))
  (UserInterface|Viewport|AddtoViewport _output_get 0))

(fn ConstructionScript
  (|CallParentFunction))

(fn UpdateMission
  (params (currentMission :type String))
  (Variables|Default|SetcurrentMission currentMission)
  (Rendering|Components|TextRender|SetText (Variables|/Game/Mechanic/Missions/WBP_Mission.WBP_Mission_C|GetcurrentMissionText (Variables|Default|GetMissionWBP)) (Utilities|Text|ToText(String) (Variables|Default|GetcurrentMission))))