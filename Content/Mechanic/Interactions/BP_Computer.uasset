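; BP_Computer is an interaction actor that activates in response to a linked Stone.
; On BeginPlay it binds to the Stone's get and destroyed events if that reference is valid.
; Getting the Stone runs ExampleTake, which fires the ComputerActivated dispatcher and destroys the computer actor.
; Stone destruction, like BeginPlay, calls ExampleLeave, which is an empty placeholder.
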(event Custom|ExampleTake
  (Default|CallComputerActivated)
  (Actor|DestroyActor))

(event Custom|ExampleLeave)

(event Custom|StoneDestroyed
  (CallFunction|ExampleLeave))

(event Custom|StoneGet
  (CallFunction|ExampleTake))

(event EventBeginPlay
  (bind _stone (Variables|Default|GetStone))
  (CallFunction|ExampleLeave)
  (Utilities|IsValid _stone
    (:Is%20Valid
      (EventDispatchers|BindEventtoStoneGet _stone (delegate Custom|StoneGet))
      (EventDispatchers|BindEventtoStoneDestroyed _stone (delegate Custom|StoneDestroyed)))))

(fn ConstructionScript)