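; BP_Drive13 is a map 13 drive pickup actor tied to a Computer interaction.
; On BeginPlay it binds DriveCreated to the computer's interacted event, if that reference is valid.
; When triggered, DriveGet broadcasts DriveAktif to listeners and destroys the actor.
; DriveDestroyed forwards to DriveLeave, which is an empty stub, and nothing in this graph binds it.
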(event Custom|DriveGet
  (Default|CallDriveAktif)
  (Actor|DestroyActor))

(event Custom|DriveLeave)

(event Custom|DriveCreated
  (CallFunction|DriveGet))

(event Custom|DriveDestroyed
  (CallFunction|DriveLeave))

(event EventBeginPlay
  (bind _computer (Variables|Default|GetComputer))
  (Utilities|IsValid _computer
    (:Is%20Valid
      (EventDispatchers|BindEventtoComputerInteracted _computer (delegate Custom|DriveCreated)))))

(fn ConstructionScript
  (|CallParentFunction))