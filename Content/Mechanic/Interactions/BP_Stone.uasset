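; BP_Stone is an interactable stone actor that removes itself when picked up and fires a StoneGet dispatcher.
; BeginPlay applies its Material variable to the static mesh.
; Interact sets the Get flag, then passes a DoN gate limited to two runs into a branch on that flag.
; Because Get is always true there, the alternate StoneDestroyed dispatch is unreachable through this path.
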(event EventBeginPlay
  (Rendering|Material|SetMaterial (Variables|Default|GetStaticMesh) 0 (Variables|Default|GetMaterial)))

(event EventInteract
  (Variables|Default|SetGet true)
  (Utilities|FlowControl|DoN 2
    (:Exit
      (if (Variables|Default|GetGet)
        (Variables|Default|SetGet false)
        (Actor|DestroyActor)
        (Default|CallStoneGet)
        (else
          (Variables|Default|SetGet true)
          (Default|CallStoneDestroyed))))))

(fn ConstructionScript
  (|CallParentFunction))