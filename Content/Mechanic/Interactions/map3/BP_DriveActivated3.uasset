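; BP_DriveActivated3 is a map 3 interactable that responds to a referenced Drive's activation and serves as a level transition.
; On BeginPlay it binds to the Drive's DriveAktif event, which shifts its static mesh upward by a fixed offset.
; Interact shows the maps transition widget, opens the level named by Map, then stores that map in SpaceGameInstance and saves the game.
; Interact itself does not check whether the Drive has activated.
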(event Custom|DriveTransform
  (Transformation|AddWorldOffset (Variables|Default|GetStaticMesh) "0.000000,0.000000,376.000000" false false))

(event EventBeginPlay
  (bind _drive (Variables|Default|GetDrive))
  (Utilities|IsValid _drive
    (:Is%20Valid
      (EventDispatchers|BindEventtoDriveAktif _drive (delegate Custom|DriveTransform)))))

(event EventInteract
  (bind _returnvalue (UserInterface|CreateWidget "/Game/Mechanic/Widget/WBP_MapsTransition.WBP_MapsTransition_C"))
  (UserInterface|Viewport|AddtoViewport _returnvalue 0)
  (Game|OpenLevel(byName) (Variables|Default|GetMap))
  (bind _asspace_game_instance (Utilities|Casting|CastToSpaceGameInstance (Game|GetGameInstance)))
  (Variables|/Game/Mechanic/Core/SpaceGameInstance.SpaceGameInstance_C|SetMap _asspace_game_instance (Variables|Default|GetMap))
  (Default|SaveGame _asspace_game_instance))

(fn ConstructionScript
  (|CallParentFunction))