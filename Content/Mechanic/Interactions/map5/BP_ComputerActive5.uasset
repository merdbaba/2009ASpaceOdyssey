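; Interactable map 5 computer that shows a WBP_Map5 widget and stays linked to a referenced Computer actor.
; When that Computer fires its activated event, this actor's static mesh moves up 396 units.
; Interact toggles the widget: one use creates it and adds it to the viewport, the next removes it and calls ComputerInteracted.
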(event Custom|ComputerCreated
  (Class|SceneComponent|AddWorldTransform (Variables|Default|GetStaticMesh) (Math|Transform|MakeTransform "0.000000,0.000000,396.000000" "0, 0, 0" "1.000000,1.000000,1.000000") false false))

(event EventBeginPlay
  (bind _computer (Variables|Default|GetComputer))
  (Variables|Default|SetWidget true)
  (Utilities|IsValid _computer
    (:Is%20Valid
      (EventDispatchers|BindEventtoComputerActivated _computer (delegate Custom|ComputerCreated)))))

(event EventInteract
  (if (Variables|Default|GetWidget)
    (Variables|Default|SetWidget false)
    (Development|PrintString "Success")
    (bind _returnvalue (UserInterface|CreateWidget "/Game/Mechanic/Widget/WBP_Map5.WBP_Map5_C"))
    (UserInterface|Viewport|AddtoViewport _returnvalue 0)
    (else
      (Variables|Default|SetWidget true)
      (Development|PrintString "Failed")
      (Widget|RemovefromParent _returnvalue)
      (Default|CallComputerInteracted))))

(fn ConstructionScript
  (|CallParentFunction))